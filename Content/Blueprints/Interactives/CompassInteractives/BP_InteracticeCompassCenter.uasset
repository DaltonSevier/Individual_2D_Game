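; Center compass interactable that acts as the win trigger once the player has collected the other compass pieces.
; Interact checks the player's CompassCollection for the NorthEast, NorthWest, SouthEast and SouthWest entries; otherwise nothing happens.
; When all four are set, it marks the center entry and destroys itself.
; It then disables input, plays a victory sound and displays the WBP_YouWin widget with the mouse cursor visible.
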(event EventBeginPlay
  (|CallParentFunction) ; This node is disabled and will not be called.\nDrag off pins to build functionality.
)

(event Collision|EventActorBeginOverlap
  (params (OtherActor :type Actor%20Object%20Reference)))

(event EventTick
  (params (DeltaSeconds :type Float%20%28single-precision%29)))

(fn ConstructionScript
  (|CallParentFunction))

(fn Interact
  (params (PlayerRef :type BP%20Player%20Base%20Object%20Reference))
  (bind _returnvalue (Game|GetPlayerController 0))
  (if (Math|Boolean|ANDBoolean (Math|Boolean|Equal(Boolean) (Utilities|Array|Get(acopy) (Variables|/Game/Blueprints/BP_PlayerBase.BP_PlayerBase_C|GetCompassCollection PlayerRef) (Variables|Default|GetNorthEastIndex)) true) (Math|Boolean|Equal(Boolean) (Utilities|Array|Get(acopy) (Variables|/Game/Blueprints/BP_PlayerBase.BP_PlayerBase_C|GetCompassCollection PlayerRef) (Variables|Default|GetNorthWestIndex)) true) (Math|Boolean|Equal(Boolean) (Utilities|Array|Get(acopy) (Variables|/Game/Blueprints/BP_PlayerBase.BP_PlayerBase_C|GetCompassCollection PlayerRef) (Variables|Default|GetSouthEastIndex)) true) (Math|Boolean|Equal(Boolean) (Utilities|Array|Get(acopy) (Variables|/Game/Blueprints/BP_PlayerBase.BP_PlayerBase_C|GetCompassCollection PlayerRef) (Variables|Default|GetSouthWestIndex)) true))
    ;[1 1 1] Sets boolean for North index to true
    (Utilities|Array|SetArrayElem (Variables|/Game/Blueprints/BP_PlayerBase.BP_PlayerBase_C|GetCompassCollection PlayerRef) (Variables|Default|GetCenter%20Index) true)
    (Actor|DestroyActor)
    (Input|DisableInput (Game|GetPlayerController 0) 0)
    (Audio|PlaySoundatLocation "/Game/Assets/Sounds/VictorySound.VictorySound" "0, 0, 0" "0, 0, 0" 1.0 1.0 0.0 0 0 0)
    (bind _returnvalue_2 (UserInterface|CreateWidget "/Game/Blueprints/UI/WBP_YouWin.WBP_YouWin_C"))
    (UserInterface|Viewport|AddtoViewport _returnvalue_2 0)
    (Input|SetInputModeGameOnly _returnvalue)
    (Variables|/Script/Engine.PlayerController|SetbShowMouseCursor _returnvalue true)))