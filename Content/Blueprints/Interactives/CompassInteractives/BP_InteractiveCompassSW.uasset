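; BP_InteractiveCompassSW is an interactive compass pickup for the SouthWest direction, gated on the player already holding South and West.
; Interact checks the South and West flags in the player's CompassCollection array, then sets the SouthWest flag and destroys the actor.
; Print strings report the acquisition or the missing prerequisites.
; BeginPlay, overlap and Tick are unused.
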(event EventBeginPlay
  (|CallParentFunction) ; This node is disabled and will not be called.\nDrag off pins to build functionality.
)

(event Collision|EventActorBeginOverlap
  (params (OtherActor :type Actor%20Object%20Reference)))

(event EventTick
  (params (DeltaSeconds :type Float%20%28single-precision%29)))

(fn ConstructionScript
  (|CallParentFunction))

(fn Interact
  (params (PlayerRef :type BP%20Player%20Base%20Object%20Reference))
  (if (and (Math|Boolean|Equal(Boolean) (Utilities|Array|Get(acopy) (Variables|/Game/Blueprints/BP_PlayerBase.BP_PlayerBase_C|GetCompassCollection PlayerRef) (Variables|Default|GetSouthIndex)) true) (Math|Boolean|Equal(Boolean) (Utilities|Array|Get(acopy) (Variables|/Game/Blueprints/BP_PlayerBase.BP_PlayerBase_C|GetCompassCollection PlayerRef) (Variables|Default|GetWestIndex)) true))
    ;[1 1 1] Sets boolean for North index to true
    (Utilities|Array|SetArrayElem (Variables|/Game/Blueprints/BP_PlayerBase.BP_PlayerBase_C|GetCompassCollection PlayerRef) (Variables|Default|GetSouthWestIndex) true)
    (Actor|DestroyActor)
    (Development|PrintString (Utilities|String|ToString(Boolean) (Utilities|Array|Get(acopy) (Variables|/Game/Blueprints/BP_PlayerBase.BP_PlayerBase_C|GetCompassCollection PlayerRef) (Variables|Default|GetSouthWestIndex))))
    (Development|PrintString "SouthWest Acquired")
    (else
      (Development|PrintString "Need South and West"))))